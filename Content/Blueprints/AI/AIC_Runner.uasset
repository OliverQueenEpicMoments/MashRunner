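; AI controller that drives a BP_Runner pawn by faking alternating left and right power inputs.
; On possess it caches the runner; BeginPlay starts a timer with a random delay between min and max bounds.
; A FlipFlop in SimulateInput alternates the two power calls and restarts the timer each time, giving a self-sustaining input loop with irregular timing.
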(event Custom|SimulateInput
  (bind _owningrunner (Variables|Default|GetOwningRunner))
  (Utilities|FlowControl|FlipFlop
    (:A
      (Default|SimulatePowerLeft _owningrunner)
      (CallFunction|SimulateDelayedInput))
    (:B
      (Default|SimulatePowerRight _owningrunner)
      (CallFunction|SimulateDelayedInput))))

(event EventBeginPlay
  (CallFunction|SimulateDelayedInput))

(event EventPossess
  (params (PossessedPawn :type Pawn%20Object%20Reference))
  (bind _asbp_runner (Utilities|Casting|CastToBP_Runner PossessedPawn))
  (Variables|Default|SetOwningRunner _asbp_runner))

(fn ConstructionScript)

(fn SimulateDelayedInput
  (Utilities|Time|SetTimerbyEvent (EventDispatchers|CreateEvent :!event Custom|SimulateInput) (Math|Random|RandomFloatinRange (Variables|Default|GetMinInputDelay) (Variables|Default|GetMaxInputDelay))))